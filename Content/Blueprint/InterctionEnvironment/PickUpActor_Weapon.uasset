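; Weapon pickup actor that gives its weapon to the inventory of an overlapping character.
; On BeginPlay it looks up WeaponInfo by ItemName through the game instance, or uses the existing value, then keeps either the static or skeletal mesh component.
; If the inventory takes the weapon the pickup succeeds; otherwise it starts a weapon switch on BP_Character, which ends when that character leaves the sphere.
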(event `self.ReceiveBeginPlay`
  (bind _itemname (`self.ItemName`))
  (`parent.ReceiveBeginPlay`)
  (if (!= _itemname "None")
    (bind _asbp_game_instanse (cast `/Game/Blueprint/Game/BP_GAMEINSTANSE` (`GameplayStatics.GetGameInstance`)))
    (bind (_outinfo _returnvalue) (`TPSGameInstance.GetDropItemInfoByName` _asbp_game_instanse _itemname))
    (if _returnvalue
      (set `self.WeaponInfo` _outinfo)))
  (`self.InitActor` (`self.WeaponInfo`)))

(event `self.OverlapCharacter`
  (params (ToInventor :type "TPSInventoryComponent Object Reference"))
  (`parent.OverlapCharacter` ToInventor)
  (bind _returnvalue (`TPSInventoryComponent.TryGetWeaponToInventory` ToInventor (`.WeaponInfo` (break `DropItem` (`self.WeaponInfo`)))))
  (if _returnvalue
    (`self.PickUPSuccess`)
    (else
      (bind _asbp_character (cast `/Game/Blueprint/Character/BP_Character` (`ActorComponent.GetOwner` ToInventor)))
      (`/Game/Blueprint/Character/BP_Character.StartSwithsWeapon` _asbp_character self))))

(event `self.Sphere.OnComponentEndOverlap`
  (params (OverlappedComponent :type "PrimitiveComponent Object Reference") (OtherActor :type "Actor Object Reference") (OtherComp :type "PrimitiveComponent Object Reference") (OtherBodyIndex :type Integer))
  (bind _asbp_character (cast `/Game/Blueprint/Character/BP_Character` OtherActor))
  (`/Game/Blueprint/Character/BP_Character.EndSweithcWeapon` _asbp_character))

(fn `InitActor`
  (params (InfoActor :type "DropItem Structure"))
  (bind (_weaponstaticmesh _weaponskeletmesh _weaponinfo) (break `DropItem` InfoActor))
  (`/Engine/EditorBlueprintResources/StandardMacros.IsValid` _weaponstaticmesh
    (:`Is Valid`
      (`ActorComponent.K2_DestroyComponent` (`self.SkeletalMesh`))
      (`StaticMeshComponent.SetStaticMesh` (`self.StaticMesh`) _weaponstaticmesh))
    (:`Is Not Valid`
      (`/Engine/EditorBlueprintResources/StandardMacros.IsValid` _weaponskeletmesh
        (:`Is Valid`
          (`ActorComponent.K2_DestroyComponent` (`self.StaticMesh`))
          (`SkinnedMeshComponent.SetSkinnedAssetAndUpdate` (`self.SkeletalMesh`) _weaponskeletmesh true))
        (:`Is Not Valid`
          (`KismetSystemLibrary.PrintString` "Error Drop Mesh"))))))

(fn `UserConstructionScript`
  (`parent.UserConstructionScript`))