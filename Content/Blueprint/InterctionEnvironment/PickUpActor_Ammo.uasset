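; Ammo pickup actor that gives a character ammunition of a set weapon type.
; Extends a parent pickup class, overriding its character overlap event, which supplies the inventory to receive the ammo.
; If that inventory can take the ammo type, it adds the pickup's count to the matching slot and calls the pickup success handler.
; InitActor runs on BeginPlay but has an empty body here.
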(event `self.ReceiveBeginPlay`
  (`parent.ReceiveBeginPlay`)
  (`self.InitActor` (struct)))

(event `self.OverlapCharacter`
  (params (ToInventor :type "TPSInventoryComponent Object Reference"))
  (bind _weapontypeammo (`self.WeaponTypeAmmo`))
  (`parent.OverlapCharacter` ToInventor)
  (bind _returnvalue (`TPSInventoryComponent.CheckCanTakeAmmo` ToInventor _weapontypeammo))
  (if _returnvalue
    (`TPSInventoryComponent.AmmoSlotChangeValue` ToInventor _weapontypeammo (`self.Cout`))
    (`self.PickUPSuccess`)))

(fn `InitActor`
  (params (InfoActor :type "DropItem Structure")))

(fn `UserConstructionScript`
  (`parent.UserConstructionScript`))